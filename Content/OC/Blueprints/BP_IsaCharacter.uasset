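; Player character Blueprint handling sprint, pause menu, world interaction, physics grabbing and ragdoll death.
; BeginPlay activates the third-person camera, starts music and creates health, minimap, map book and keypad clue widgets, with both books toggled by input.
; Interactions use a line trace or sphere trace to send interface messages.
; E grabs traced components through a PhysicsHandle, which a retriggerable-delay loop, replacing Tick, holds ahead of the first-person camera.
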(event `TraceForLock`
  ; Not sure if I need this?
  (bind (_location _rotation) (`self.GetPlayerViewPoint`)))

(event `EnhancedInput|/Game/ThirdPerson/Input/Actions/IA_Pausegame`
  (params (ActionValue :type Boolean) (ElapsedSeconds :type "Float (double-precision)") (TriggeredSeconds :type "Float (double-precision)") (InputAction :type "InputAction Object Reference" :default "/Game/ThirdPerson/Input/Actions/IA_Pausegame.IA_Pausegame"))
  (bind _returnvalue (`GameplayStatics.GetPlayerController` 0))
  ;[0.15 0.02491 0.1261 0.5] Pause Menu
  (:`Started`
    (`GameplayStatics.PlaySound2D` "/Game/UI_PAUSEMENU/Audio/A_Widgetopen.A_Widgetopen" 1.0 1.0 0.0 null null)
    (if (not (`self.IsPauseMenuOpen?`))
      (set `self.IsPauseMenuOpen?` true)
      (bind _returnvalue_2 (`|CreateWidget` "/Game/OC/Widgets/WB_Mainmenu.WB_Mainmenu_C" _returnvalue))
      (bind _output_get (set `self.Pause Menu Widget` _returnvalue_2))
      (`UserWidget.AddToViewport` _output_get 0)
      (`WidgetBlueprintLibrary.SetInputMode_GameAndUIEx` _returnvalue (`self.Pause Menu Widget`))
      (set `PlayerController.bShowMouseCursor` true (`GameplayStatics.GetPlayerController` 0))
      (`GameplayStatics.SetGamePaused` true)
      (`KismetSystemLibrary.PrintString` "Hello dude")
      (else
        (set `self.IsPauseMenuOpen?` false)
        (`Widget.RemoveFromParent` (`self.Pause Menu Widget`))
        (`GameplayStatics.SetGamePaused` false)
        (`WidgetBlueprintLibrary.SetInputMode_GameOnly` _returnvalue)
        (set `PlayerController.bShowMouseCursor` false (`GameplayStatics.GetPlayerController` 0))))))

(event `self.ReceiveBeginPlay`
  ;[0.01631 0.04868 0.15 0.5] Set Active Camera to Third person camera on Begin play
  (`|ExecutionSequence`
    (:`then_0`
      (`ActorComponent.SetActive` (`self.ThirdPersonCamera`) true false)
      (`ActorComponent.SetActive` (`self.FirstPersonCamera`) false false)
      (set `self.bUseControllerRotationYaw` false)
      (`GameplayStatics.SpawnSound2D` "/Game/OC/Sounds/lights-of-morocco-258597.lights-of-morocco-258597" 1.0 1.0 0.0 null))
    (:`then_1`
      ;[0.04737 0.15 0.02053 0.5] Health Bar Ui
      (bind _returnvalue (`|CreateWidget` "/Game/OC/Widgets/HealthBar.HealthBar_C"))
      (`UserWidget.AddToViewport` _returnvalue 0)
      ; MapBook Widget UI(Hidden untill
      (bind _returnvalue_2 (`|CreateWidget` "/Game/OC/Widgets/WBP_Book.WBP_Book_C"))
      (bind _output_get (set `self.OpenBookWidget` _returnvalue_2))
      (`UserWidget.AddToViewport` _output_get 0)
      (`Widget.SetVisibility` _output_get "Hidden")
      ; MiniMap Widget
      (bind _returnvalue_3 (`|CreateWidget` "/Game/OC/Widgets/WBP_MiniMap.WBP_MiniMap_C" (`GameplayStatics.GetPlayerController` 0)))
      (`UserWidget.AddToViewport` _returnvalue_3 0)
      ; Keypad Clue Widget
      (bind _returnvalue_4 (`|CreateWidget` "/Game/OC/Widgets/WBP_Book_KeypadClue.WBP_Book_KeypadClue_C"))
      (bind _output_get_2 (set `self.OpenBook_KeyPadClueWidget` _returnvalue_4))
      (`UserWidget.AddToViewport` _output_get_2 0)
      (`Widget.SetVisibility` _output_get_2 "Hidden"))
    (:`then_2`
      ; Tick to call PickUpObjects Event
      (`self.Timer_PickUpObject`))))

(event `InputActionFire`
  (params (Pressed :type Boolean))
  ; InteractionControl
  (if (not (`self.UsingLock?`))
    (`self.InputActionFire` false)))

(event `EnhancedInput|/Game/ThirdPerson/Input/Actions/IA_Run`
  (params (ActionValue :type Boolean) (ElapsedSeconds :type "Float (double-precision)") (TriggeredSeconds :type "Float (double-precision)") (InputAction :type "InputAction Object Reference" :default "/Game/ThirdPerson/Input/Actions/IA_Run.IA_Run"))
  (bind _charactermovement (`self.CharacterMovement`))
  ;[0.15 0.1234 0.001538 0.5] Run_Left Shift Key
  (:`Started`
    (set `CharacterMovementComponent.MaxWalkSpeed` 500.0 _charactermovement))
  (:`Completed`
    (set `CharacterMovementComponent.MaxWalkSpeed` 200.0 _charactermovement)))

(event `EnhancedInput|/Game/ThirdPerson/Input/Actions/Ia_Interact`
  (params (ActionValue :type Boolean) (ElapsedSeconds :type "Float (double-precision)") (TriggeredSeconds :type "Float (double-precision)") (InputAction :type "InputAction Object Reference" :default "/Game/ThirdPerson/Input/Actions/Ia_Interact.Ia_Interact"))
  ;[0.15 0.07406 0.1416 0.5] IA_Interact Draw Line Trace for Interactions
  (:`Started`
    (`self.LineTrace`)))

(event `LineTrace`
  (bind _firstpersoncameraboom (`self.FirstPersonCameraBoom`))
  (bind _returnvalue (`SceneComponent.K2_GetComponentLocation` _firstpersoncameraboom))
  ;[0.1474 0.07031 0.15 0.5] Blueprint Interface / Line Trace
  (bind (_outhit _returnvalue_2) (`KismetSystemLibrary.LineTraceSingle` :`Start` _returnvalue :`End` (+ _returnvalue (* (`SceneComponent.GetForwardVector` _firstpersoncameraboom) 250.0)) :`TraceChannel` "TraceTypeQuery1" :`DrawDebugType` "Persistent"))
  (if _returnvalue_2
    (bind (_bblockinghit _binitialoverlap _time _distance _location _impactpoint _normal _impactnormal _physmat _hitactor) (`GameplayStatics.BreakHitResult` _outhit))
    (if (`KismetSystemLibrary.DoesImplementInterface` _hitactor "/Game/OC/Blueprints/Interfaces/UseOpenClose.UseOpenClose_C")
      (message `/Game/OC/Blueprints/Interfaces/UseOpenClose.UseOpenClose` _hitactor))))

(event `EnhancedInput|/Game/ThirdPerson/Input/Actions/IA_OpenSluice`
  (params (ActionValue :type Boolean) (ElapsedSeconds :type "Float (double-precision)") (TriggeredSeconds :type "Float (double-precision)") (InputAction :type "InputAction Object Reference" :default "/Game/ThirdPerson/Input/Actions/IA_OpenSluice.IA_OpenSluice"))
  (bind _returnvalue (`self.K2_GetActorLocation`))
  ;[0 0.81 0.9167 0.5] Open Sluice Gate Interact with E Key
  (:`Triggered`
    (bind (_outhits _returnvalue_2) (`KismetSystemLibrary.SphereTraceMulti` _returnvalue _returnvalue 200.0 "TraceTypeQuery1"))
    (if _returnvalue_2
      (message `/Game/OC/Blueprints/Interfaces/BPI_Interact.InteractEvent` (`.HitActor` (`GameplayStatics.BreakHitResult` (`|GetArrayItem` _outhits)))))))

(event `Death`
  ;[0.15 0.05393 0.03595 0.5] Ragdoll Collision
  (`PrimitiveComponent.SetSimulatePhysics` (`self.Mesh`) true))

(event `Key|E`
  (params (Key :type "Key Structure"))
  (bind _firstpersoncamera (`self.FirstPersonCamera`))
  (bind _returnvalue (`SceneComponent.K2_GetComponentLocation` _firstpersoncamera))
  ;[0.15 0.1369 0.05092 0.595] Grabbing System - E Key
  (:`Pressed`
    (bind (_outhit _returnvalue_2) (`KismetSystemLibrary.LineTraceSingle` :`Start` _returnvalue :`End` (+ _returnvalue (* (`KismetMathLibrary.GetForwardVector` (`SceneComponent.K2_GetComponentRotation` _firstpersoncamera)) 200.0)) :`TraceChannel` "TraceTypeQuery1" :`DrawDebugType` "ForDuration"))
    (if _returnvalue_2
      (bind (_bblockinghit _binitialoverlap _time _distance _location _impactpoint _normal _impactnormal _physmat _hitactor _hitcomponent) (`GameplayStatics.BreakHitResult` _outhit))
      (`PhysicsHandleComponent.GrabComponentAtLocationWithRotation` :`self` (`self.PhysicsHandle`) :`Component` _hitcomponent :`Location` (`SceneComponent.K2_GetComponentLocation` _hitcomponent))
      (set `self.IsGrabbingObject?` true)))
  (:`Released`
    (if (`self.IsGrabbingObject?`)
      (`PhysicsHandleComponent.ReleaseComponent` (`self.PhysicsHandle`))
      (set `self.IsGrabbingObject?` false))))

(event `Timer_PickUpObject`
  ;[0.15 0.1369 0.05092 0.595] Delay forPickUpObjects Event (Replace Tick)
  (`self.PickUPObjects` :!label _label)
  (`KismetSystemLibrary.RetriggerableDelay` (`self.Delay_PickUpObjects`))
  (goto _label))

(event `PickUPObjects`
  (bind _firstpersoncamera (`self.FirstPersonCamera`))
  ;[0.15 0.1369 0.05092 0.595] Object Picked Up Loop
  (if (`self.IsGrabbingObject?`)
    (`PhysicsHandleComponent.SetTargetLocation` (`self.PhysicsHandle`) (+ (`SceneComponent.K2_GetComponentLocation` _firstpersoncamera) (* (`KismetMathLibrary.GetForwardVector` (`SceneComponent.K2_GetComponentRotation` _firstpersoncamera)) 200)))))

(event `EnhancedInput|/Game/ThirdPerson/Input/Actions/IA_OpenBook`
  (params (ActionValue :type Boolean) (ElapsedSeconds :type "Float (double-precision)") (TriggeredSeconds :type "Float (double-precision)") (InputAction :type "InputAction Object Reference" :default "/Game/ThirdPerson/Input/Actions/IA_OpenBook.IA_OpenBook"))
  (bind _openbookwidget (`self.OpenBookWidget`))
  ;[0.01652 0.03509 0.15 0.5] OpenMapBook X key
  (:`Triggered`
    (`/Engine/EditorBlueprintResources/StandardMacros.FlipFlop`
      (:`A`
        (`Widget.SetVisibility` _openbookwidget "Visible"))
      (:`B`
        (`Widget.SetVisibility` _openbookwidget "Hidden")))))

(event `EnhancedInput|/Game/ThirdPerson/Input/Actions/IA_OpenBook_KeyPadClue`
  (params (ActionValue :type Boolean) (ElapsedSeconds :type "Float (double-precision)") (TriggeredSeconds :type "Float (double-precision)") (InputAction :type "InputAction Object Reference" :default "/Game/ThirdPerson/Input/Actions/IA_OpenBook_KeyPadClue.IA_OpenBook_KeyPadClue"))
  (bind _openbook_keypadcluewidget (`self.OpenBook_KeyPadClueWidget`))
  ;[0.01652 0.03509 0.15 0.5] OpenKeypadBook R key
  (:`Triggered`
    (`/Engine/EditorBlueprintResources/StandardMacros.FlipFlop`
      (:`A`
        (`Widget.SetVisibility` _openbook_keypadcluewidget "Visible"))
      (:`B`
        (`Widget.SetVisibility` _openbook_keypadcluewidget "Hidden")))))

(fn `GetPlayerViewPoint`
  (returns (Location :type "Vector Structure") (Rotation :type "Rotator Structure"))
  (return (0.0 0.0 0.0)))

(fn `Isinteractable`
  (returns (Interactable :type Boolean))
  (return false))

(fn `UserConstructionScript`)