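; Wall keypad actor that shows a code lock widget when used and opens doors once the correct code is entered.
; Interface use toggles WBP_CodeLock with its cursor and input mode, and leaving the Box volume closes it.
; The widget's success event blocks reopening, then after a delay calls OpenDoor on every BP_DoorSwing in the level.
; A separate hint volume shows and hides an interact prompt for the player.
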(event `/Game/OC/Blueprints/Interfaces/UseOpenClose.UseOpenClose`
  ;[0.15 0.1138 0.03916 0.5] Blueprint Interface Command
  (`self.Toggle Door Code`))

(event `Toggle Door Code`
  ;[0.02084 0.03085 0.15 0.5] Toggle Widget on Screen
  (if (`self.Is On Screen?`)
    (`self.Close Code Lock`)
    (else
      (`self.Use Code Lock`))))

(event `Use Code Lock`
  (bind _returnvalue (`GameplayStatics.GetPlayerController` 0))
  ; Correct code has been recieved, play animatin for door and block all input for displaying widget
  (if (not (`self.CorrectInputEntered?`))
    (bind _returnvalue_2 (`|CreateWidget` "/Game/OC/Widgets/WBP_CodeLock.WBP_CodeLock_C" _returnvalue))
    (bind _output_get (set `self.WallPad_Widget` _returnvalue_2))
    (set `/Game/OC/Widgets/WBP_CodeLock.Correct Code` (`self.Correct Code`) _output_get)
    (`UserWidget.AddToViewport` _output_get 0)
    (`WidgetBlueprintLibrary.SetInputMode_GameAndUIEx` _returnvalue _output_get)
    (set `PlayerController.bShowMouseCursor` true _returnvalue)
    (set `self.Is On Screen?` true)
    ;[0.1001 0.15 0.07111 0.5] Correct input code achieved
    (add `/Game/OC/Widgets/WBP_CodeLock.Correct Input added` _output_get (delegate `Correct Input Open Door`))))

(event `Correct Input Open Door`
  ;[0.1001 0.15 0.07111 0.5] Correct input code achieved
  (set `self.CorrectInputEntered?` true)
  (`KismetSystemLibrary.Delay` 2.0)
  (`GameplayStatics.GetAllActorsOfClass` "/Game/OC/Blueprints/Keypad/BP_DoorSwing.BP_DoorSwing_C")
  (for _array_element (`self.Out Actors`)
    (`/Game/OC/Blueprints/Keypad/BP_DoorSwing.Open door` _array_element)))

(event `Close Code Lock`
  (bind _returnvalue (`GameplayStatics.GetPlayerController` 0))
  ;[0.02175 0.1026 0.15 0.5] Close Widget Codelock remove from screen/ remove from screen if player moves away
  (`Widget.RemoveFromParent` (`self.WallPad_Widget`) :!label _label)
  (`WidgetBlueprintLibrary.SetInputMode_GameOnly` _returnvalue)
  (set `PlayerController.bShowMouseCursor` false _returnvalue)
  (set `self.Is On Screen?` false))

(event `self.Box.OnComponentEndOverlap`
  (params (OverlappedComponent :type "PrimitiveComponent Object Reference") (OtherActor :type "Actor Object Reference") (OtherComp :type "PrimitiveComponent Object Reference") (OtherBodyIndex :type Integer))
  ;[0.02175 0.1026 0.15 0.5] Close Widget Codelock remove from screen/ remove from screen if player moves away
  (goto _label))

(event `self.ReceiveBeginPlay`
  (bind _returnvalue (`|CreateWidget` "/Game/OC/Widgets/Prompt_Interact.Prompt_Interact_C"))
  (set `self.Interact_Promt` _returnvalue))

(event `self.Box_Hint.OnComponentBeginOverlap`
  (params (OverlappedComponent :type "PrimitiveComponent Object Reference") (OtherActor :type "Actor Object Reference") (OtherComp :type "PrimitiveComponent Object Reference") (OtherBodyIndex :type Integer) (bFromSweep :type Boolean) (SweepResult :type "HitResult Structure (by ref)"))
  (if (== OtherActor (`GameplayStatics.GetPlayerCharacter` 0))
    (`UserWidget.AddToViewport` (`self.Interact_Promt`) 0)))

(event `self.Box_Hint.OnComponentEndOverlap`
  (params (OverlappedComponent :type "PrimitiveComponent Object Reference") (OtherActor :type "Actor Object Reference") (OtherComp :type "PrimitiveComponent Object Reference") (OtherBodyIndex :type Integer))
  (if (== (`GameplayStatics.GetPlayerCharacter` 0) OtherActor)
    (`Widget.RemoveFromParent` (`self.Interact_Promt`))))

(fn `UserConstructionScript`)