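; BP_Door is a keypad-locked door that opens when the player enters the correct code.
; An interface event toggles the WBP_CodeLock widget, passing it the door's code and switching input to Game and UI with a visible cursor.
; The widget's correct-input event marks the door solved, then after a delay a timeline rotates it open with sounds.
; Closing the keypad or leaving the box overlap removes all widgets and restores game-only input.
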(event `/Game/OC/Blueprints/Interfaces/UseOpenClose.UseOpenClose`
  ;[0.15 0.1138 0.03916 0.5] Blueprint Interface Command
  (`self.Toggle Door Code`))

(event `Toggle Door Code`
  ;[0.02084 0.03085 0.15 0.5] Toggle Widget on Screen
  (if (`self.Is On Screen?`)
    (`self.Close Code Lock`)
    (else
      (`self.Use Code Lock`))))

(event `Use Code Lock`
  (bind _returnvalue (`GameplayStatics.GetPlayerController` 0))
  ; Correct code has been recieved, play animatin for door and block all input for displaying widget
  (if (not (`self.CorrectInputEntered?`))
    (bind _returnvalue_2 (`|CreateWidget` "/Game/OC/Widgets/WBP_CodeLock.WBP_CodeLock_C" _returnvalue))
    (set `/Game/OC/Widgets/WBP_CodeLock.Correct Code` (`self.Correct Code`) _returnvalue_2)
    (`UserWidget.AddToViewport` _returnvalue_2 0)
    (`WidgetBlueprintLibrary.SetInputMode_GameAndUIEx` _returnvalue _returnvalue_2)
    (set `PlayerController.bShowMouseCursor` true _returnvalue)
    (set `self.Is On Screen?` true)
    ;[0.1001 0.15 0.07111 0.5] Correct input code achieved
    (add `/Game/OC/Widgets/WBP_CodeLock.Correct Input added` _returnvalue_2 (delegate `Correct Input Open Door`))))

(event `Correct Input Open Door`
  ;[0.1001 0.15 0.07111 0.5] Correct input code achieved
  (set `self.CorrectInputEntered?` true)
  (`KismetSystemLibrary.Delay` 4.0)
  ;; DoorOpening sound
  (`GameplayStatics.PlaySoundAtLocation` "/Game/OC/Sounds/Cues/OpenDoor.OpenDoor" (`SceneComponent.K2_GetComponentLocation` (`self.DOOR`)) (struct) 1.0 1.0 0.0 null null null null)
  (bind (_direction _door_open) (`Timeline|Door Opening` :!via `PlayFromStart`)
    (:`Update`
      (`SceneComponent.K2_SetRelativeRotation` (`self.DOOR`) (`KismetMathLibrary.MakeRotator` 0.0 _door_open) false false))
    (:`Finished`
      ;; DoorOpensEndSound
      (`GameplayStatics.PlaySoundAtLocation` null (`SceneComponent.K2_GetComponentLocation` (`self.DOOR`)) (struct) 1.0 1.0 0.0 null null null null))))

(event `Close Code Lock`
  (bind _returnvalue (`GameplayStatics.GetPlayerController` 0))
  ;[0.02175 0.1026 0.15 0.5] Close Widget Codelock remove from screen/ remove from screen if player moves away
  (`WidgetLayoutLibrary.RemoveAllWidgets` :!label _label)
  (`WidgetBlueprintLibrary.SetInputMode_GameOnly` _returnvalue)
  (set `PlayerController.bShowMouseCursor` false _returnvalue)
  (set `self.Is On Screen?` false))

(event `self.Box.OnComponentEndOverlap`
  (params (OverlappedComponent :type "PrimitiveComponent Object Reference") (OtherActor :type "Actor Object Reference") (OtherComp :type "PrimitiveComponent Object Reference") (OtherBodyIndex :type Integer))
  ;[0.02175 0.1026 0.15 0.5] Close Widget Codelock remove from screen/ remove from screen if player moves away
  (goto _label))

(fn `UserConstructionScript`)