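; Sluice gate actor that the player opens and closes by interacting with it.
; InteractEvent alternates through a FlipFlop between playing a timeline from the start and reversing it from the end, with the timeline driving the gate's relative Z location.
; A hint overlap component shows an interaction prompt widget, created at BeginPlay, while the player character is inside it.
; The Isinteractable function always returns false.
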(event `/Game/OC/Blueprints/Interfaces/BPI_Interact.InteractEvent`
  ; Open Gate
  (`/Engine/EditorBlueprintResources/StandardMacros.FlipFlop`
    (:`A`
      (bind (_direction _open_sluicegate) (`Timeline|OpenSluiceGateTimeline` :!via `PlayFromStart` :!label _label)
        (:`Update`
          (`SceneComponent.K2_SetRelativeLocation` (`self.SluiceGate`) (`KismetMathLibrary.MakeVector` 0.0 0.0 _open_sluicegate) false false))))
    (:`B`
      (goto _label :!via `ReverseFromEnd`))))

(event `self.ReceiveBeginPlay`
  ; Hint on screen
  (bind _returnvalue (`|CreateWidget` "/Game/OC/Widgets/Prompt_Interact_SluiceGate.Prompt_Interact_SluiceGate_C"))
  (set `self.Prompt_SluiceGate` _returnvalue))

(event `self.Hint_SluiceGate.OnComponentBeginOverlap`
  (params (OverlappedComponent :type "PrimitiveComponent Object Reference") (OtherActor :type "Actor Object Reference") (OtherComp :type "PrimitiveComponent Object Reference") (OtherBodyIndex :type Integer) (bFromSweep :type Boolean) (SweepResult :type "HitResult Structure (by ref)"))
  ; Hint on screen
  (if (== OtherActor (`GameplayStatics.GetPlayerCharacter` 0))
    (`UserWidget.AddToViewport` (`self.Prompt_SluiceGate`) 0)))

(event `self.Hint_SluiceGate.OnComponentEndOverlap`
  (params (OverlappedComponent :type "PrimitiveComponent Object Reference") (OtherActor :type "Actor Object Reference") (OtherComp :type "PrimitiveComponent Object Reference") (OtherBodyIndex :type Integer))
  ; Hint on screen
  (if (== (`GameplayStatics.GetPlayerCharacter` 0) OtherActor)
    (`Widget.RemoveFromParent` (`self.Prompt_SluiceGate`))))

(fn `Isinteractable`
  (returns (Interactable :type Boolean))
  (return false))

(fn `UserConstructionScript`)