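; Two-tumbler combination lock that unlocks a linked BPUnlockable when its digits match the set Combination.
; Tick polls through a one-second Delay, comparing the child tumblers' concatenated numbers to the code, then once briefly simulates physics on the lock mesh and calls Unlock.
; A configurable trigger volume toggles UsingLock on BP_LanaCharacter while overlapped.
; Tumbler starting rotations can be randomized on BeginPlay.
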(event `self.ReceiveTick`
  (params (DeltaSeconds :type "Float (single-precision)"))
  (bind _lockmesh (`self.LockMesh`))
  ; Check for correct combination
  (`KismetSystemLibrary.Delay` 1.0)
  (bind _combomatch_ (`self.CheckCombination`))
  (if _combomatch_
    (`/Engine/EditorBlueprintResources/StandardMacros.DoOnce` false
      (:`Completed`
        (set `self.LockedState` false)
        (`KismetSystemLibrary.Delay` 1.5)
        (`SkeletalMeshComponent.SetAllBodiesSimulatePhysics` _lockmesh true)
        (`KismetSystemLibrary.Delay` 0.4)
        (`/Game/OC/Blueprints/BP_Unlockable.Unlock` (`self.BP_Unlockable`))
        (`KismetSystemLibrary.Delay` 2.0)
        (`SkeletalMeshComponent.SetAllBodiesSimulatePhysics` _lockmesh false)))))

(event `self.ReceiveBeginPlay`
  ; Randomize Tumblers?
  (if (`self.RandomizeTumblerRotation?`)
    (`/Game/OC/Blueprints/BP_LockTumbler.Randomize Tumbler` (cast `/Game/OC/Blueprints/BP_LockTumbler` (`ChildActorComponent.ChildActor` (`self.BP_LockTumbler1`)) :!pure true))
    (`/Game/OC/Blueprints/BP_LockTumbler.Randomize Tumbler` (cast `/Game/OC/Blueprints/BP_LockTumbler` (`ChildActorComponent.ChildActor` (`self.BP_LockTumbler2`)) :!pure true))))

(event `self.LockTrigger.OnComponentBeginOverlap`
  (params (OverlappedComponent :type "PrimitiveComponent Object Reference") (OtherActor :type "Actor Object Reference") (OtherComp :type "PrimitiveComponent Object Reference") (OtherBodyIndex :type Integer) (bFromSweep :type Boolean) (SweepResult :type "HitResult Structure (by ref)"))
  (bind _asbp_lana_character (cast `/Game/OC/Blueprints/BP_LanaCharacter` OtherActor))
  (set `/Game/OC/Blueprints/BP_LanaCharacter.UsingLock?` true _asbp_lana_character))

(event `self.LockTrigger.OnComponentEndOverlap`
  (params (OverlappedComponent :type "PrimitiveComponent Object Reference") (OtherActor :type "Actor Object Reference") (OtherComp :type "PrimitiveComponent Object Reference") (OtherBodyIndex :type Integer))
  (bind _asbp_lana_character (cast `/Game/OC/Blueprints/BP_LanaCharacter` OtherActor))
  (set `/Game/OC/Blueprints/BP_LanaCharacter.UsingLock?` false _asbp_lana_character))

(fn `CheckCombination`
  (returns (`ComboMatch?` :type Boolean))
  (return (== (`self.Combination`) (`KismetStringLibrary.Concat_StrStr` (`KismetStringLibrary.Conv_IntToString` (`/Game/OC/Blueprints/BP_LockTumbler.TumblerNumber` (cast `/Game/OC/Blueprints/BP_LockTumbler` (`ChildActorComponent.ChildActor` (`self.BP_LockTumbler1`)) :!pure true))) (`KismetStringLibrary.Conv_IntToString` (`/Game/OC/Blueprints/BP_LockTumbler.TumblerNumber` (cast `/Game/OC/Blueprints/BP_LockTumbler` (`ChildActorComponent.ChildActor` (`self.BP_LockTumbler2`)) :!pure true)))))))

(fn `UserConstructionScript`
  (bind _locktrigger (`self.LockTrigger`))
  (`SceneComponent.SetRelativeScale3D` _locktrigger (`self.LockTriggerScale`))
  (`SceneComponent.K2_SetRelativeLocation` _locktrigger (`self.LockTriggerLocation`) false false))