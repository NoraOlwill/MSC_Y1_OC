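; BP_EnemyAI is an enemy that chases the first player and points at them with on-screen text on arrival.
; Pawn Sensing sets IsSeeingPlayer and starts FollowPlayer, which runs AI MoveTo toward the player, while Tick halts movement whenever the flag is false.
; On arrival, CanAttack and a DoOnce gate the montage and temporary text widget, timed by montage length.
; A failed move resets the DoOnce, whose reset output retries the follow.
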(event `self.ReceiveTick`
  (params (DeltaSeconds :type "Float (single-precision)"))
  ;[0.06679 0.15 0.1024 0.5] Stop Enemy follow if cant see player
  (if (not (`self.isSeeingPlayer?`))
    (`MovementComponent.StopMovementImmediately` (`self.CharacterMovement`))))

(event `self.PawnSensing.OnSeePawn`
  (params (Pawn :type "Pawn Object Reference"))
  ;[0.1262 0.0388 0.15 0.5] See Player Pawn Sensing
  (set `self.isSeeingPlayer?` true)
  (`self.FollowPlayer`))

(event `FollowPlayer`
  ;[0.1264 0.02993 0.15 0.5] Follow player
  (set `self.canAttack?` true)
  (if (`self.isSeeingPlayer?`) :!label _label
    (`|AIMoveTo` self (0.0 0.0 0.0) (`GameplayStatics.GetPlayerCharacter` 0) 120.0
      (:`OnSuccess`
        (if (`self.canAttack?`)
          (set `self.canAttack?` false)
          (`|DoOnceMultiInput` :!label _label_2
            (:`A Out`
              (bind _returnvalue (`self.PlayAnimMontage` "/Game/Characters/AI/EnemyAI_Pointing_Montage.EnemyAI_Pointing_Montage"))
              (bind _returnvalue_2 (`|CreateWidget` "/Game/OC/Widgets/WBP_EnemyText.WBP_EnemyText_C"))
              (bind _output_get (set `self.EnemyText` _returnvalue_2))
              (`UserWidget.AddToViewport` _output_get 0)
              (`KismetSystemLibrary.Delay` _returnvalue)
              (`Widget.RemoveFromParent` (`self.EnemyText`))
              (`KismetSystemLibrary.Delay` _returnvalue)
              (set `self.canAttack?` true))
            (:`Reset Out`
              (goto _label)))))
      (:`OnFail`
        (goto _label_2 :!via `Reset In`)))
    (else
      (set `self.isSeeingPlayer?` false))))

(fn `UserConstructionScript`)