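; A single combination-lock tumbler that starts at a random rotation from a preset list and spins forward on E or backward on R.
; Each direction has its own Timeline that rolls the mesh, with a DoOnce blocking repeat input in that direction until it finishes.
; NumberCheck maps the truncated angle in 36-degree steps to digits 0–9, which are printed after each spin.
; Rotation resets to zero after a full turn either way.
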(event `ShowTumblerNumber`
  ; Show Tumbler Number
  (`KismetSystemLibrary.PrintString` (`KismetStringLibrary.Concat_StrStr` "Tunbler Number: " (`KismetStringLibrary.Conv_IntToString` (`self.TumblerNumber`))) true true (struct :`G` 0.66 :`B` 1.0 :`A` 1.0) 5.0))

(event `self.ReceiveBeginPlay`
  ; Begin Play
  (if true
    (`self.Randomize Tumbler`)))

(event `Key|E`
  (params (Key :type "Key Structure"))
  (:`Pressed`
    (`self.SpinTumbler`)))

(event `Key|R`
  (params (Key :type "Key Structure"))
  (:`Pressed`
    (`self.SpinTumblerBackward`)))

(event `SpinTumbler`
  ; SpinTumbler
  (`/Engine/EditorBlueprintResources/StandardMacros.DoOnce` false :!label _label
    (:`Completed`
      (bind (_direction _alpha) (`Timeline|Timeline` :!via `PlayFromStart`)
        (:`Update`
          (bind _returnvalue (+ (`self.TumblerRotation`) _alpha))
          (`SceneComponent.K2_SetRelativeRotation` (`self.TumblerMesh`) (`KismetMathLibrary.MakeRotator` _returnvalue) false false))
        (:`Finished`
          (set `self.TumblerRotation` _returnvalue)
          (`self.NumberCheck`)
          (`self.ShowTumblerNumber`)
          (`self.SpinTumblerReset`)
          (if (>= (`self.TumblerRotation`) 360.0)
            (set `self.TumblerRotation` 0.0)))))))

(event `SpinTumblerReset`
  ; SpinTumbler
  (goto _label :!via `Reset`))

(event `SpinTumblerBackward`
  ; SpinTumbler
  (`/Engine/EditorBlueprintResources/StandardMacros.DoOnce` false :!label _label_2
    (:`Completed`
      (bind (_direction _alpha) (`Timeline|Timeline_0` :!via `PlayFromStart`)
        (:`Update`
          (bind _returnvalue (- (`self.TumblerRotation`) _alpha))
          (`SceneComponent.K2_SetRelativeRotation` (`self.TumblerMesh`) (`KismetMathLibrary.MakeRotator` _returnvalue) false false))
        (:`Finished`
          (set `self.TumblerRotation` _returnvalue)
          (`self.NumberCheck`)
          (`self.ShowTumblerNumber`)
          (`self.SpinTumblerBackwardReset`)
          (if (<= (`self.TumblerRotation`) -360.0)
            (set `self.TumblerRotation` 0.0)))))))

(event `SpinTumblerBackwardReset`
  ; SpinTumbler
  (goto _label_2 :!via `Reset`))

(fn `NewFunction`
  (params (A :type Integer))
  (returns (ReturnValue :type Integer))
  (return (`self.NewMacro` A)))

(fn `NumberCheck`
  (if (== (`KismetMathLibrary.FTrunc` (`self.TumblerRotation`)) 0)
    (set `self.TumblerNumber` 0)
    (elif (== (`KismetMathLibrary.FTrunc` (`self.TumblerRotation`)) 36)
      (set `self.TumblerNumber` 1)
      (elif (== (`KismetMathLibrary.FTrunc` (`self.TumblerRotation`)) 72)
        (set `self.TumblerNumber` 2)
        (elif (== (`KismetMathLibrary.FTrunc` (`self.TumblerRotation`)) 108)
          (set `self.TumblerNumber` 3)
          (elif (== (`KismetMathLibrary.FTrunc` (`self.TumblerRotation`)) 144)
            (set `self.TumblerNumber` 4)
            (elif (== (`KismetMathLibrary.FTrunc` (`self.TumblerRotation`)) 180)
              (set `self.TumblerNumber` 5)
              (elif (== (`KismetMathLibrary.FTrunc` (`self.TumblerRotation`)) 216)
                (set `self.TumblerNumber` 6)
                (elif (== (`KismetMathLibrary.FTrunc` (`self.TumblerRotation`)) 252)
                  (set `self.TumblerNumber` 7)
                  (elif (== (`KismetMathLibrary.FTrunc` (`self.TumblerRotation`)) 288)
                    (set `self.TumblerNumber` 8)
                    (elif (== (`KismetMathLibrary.FTrunc` (`self.TumblerRotation`)) 324)
                      (set `self.TumblerNumber` 9)
                      (elif (== (`KismetMathLibrary.FTrunc` (`self.TumblerRotation`)) 360)
                        (set `self.TumblerNumber` 0)
                        (elif (== (`KismetMathLibrary.FTrunc` (`self.TumblerRotation`)) -36)
                          (set `self.TumblerNumber` 9)
                          (elif (== (`KismetMathLibrary.FTrunc` (`self.TumblerRotation`)) -72)
                            (set `self.TumblerNumber` 8)
                            (elif (== (`KismetMathLibrary.FTrunc` (`self.TumblerRotation`)) -108)
                              (set `self.TumblerNumber` 7)
                              (elif (== (`KismetMathLibrary.FTrunc` (`self.TumblerRotation`)) -144)
                                (set `self.TumblerNumber` 6)
                                (elif (== (`KismetMathLibrary.FTrunc` (`self.TumblerRotation`)) -180)
                                  (set `self.TumblerNumber` 5)
                                  (elif (== (`KismetMathLibrary.FTrunc` (`self.TumblerRotation`)) -216)
                                    (set `self.TumblerNumber` 4)
                                    (elif (== (`KismetMathLibrary.FTrunc` (`self.TumblerRotation`)) -252)
                                      (set `self.TumblerNumber` 3)
                                      (elif (== (`KismetMathLibrary.FTrunc` (`self.TumblerRotation`)) -288)
                                        (set `self.TumblerNumber` 2)
                                        (elif (== (`KismetMathLibrary.FTrunc` (`self.TumblerRotation`)) -324)
                                          (set `self.TumblerNumber` 1)
                                          (elif (== (`KismetMathLibrary.FTrunc` (`self.TumblerRotation`)) -360)
                                            (set `self.TumblerNumber` 0)))))))))))))))))))))))

(fn `Randomize Tumbler`
  (bind _randomrotations (`self.RandomRotations`))
  (bind _output_get (set `self.TumblerRotation` (`|GetArrayItem` _randomrotations (`KismetMathLibrary.RandomIntegerInRange` 0 (- (`KismetArrayLibrary.Array_Length` _randomrotations) 1)))))
  (`SceneComponent.K2_SetRelativeRotation` (`self.TumblerMesh`) (`KismetMathLibrary.MakeRotator` _output_get) false false)
  (`self.NumberCheck`))

(fn `UserConstructionScript`)