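; BP_old_book_KeyPadClue is an old book keypad clue actor that shows an interaction prompt when the player is near.
; On BeginPlay it creates the open-book prompt widget and stores it.
; Its Box component adds the widget to the viewport when the player character begins overlap and removes it when overlap ends.
; A graph comment names R as the open/close key, but this Blueprint handles only the prompt's visibility.
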(event `self.ReceiveBeginPlay`
  ; Prompt On screen R to open and close
  (bind _returnvalue (`|CreateWidget` "/Game/OC/Widgets/WBP_Prompt_Interact_OpenBook_KeyPadClue.WBP_Prompt_Interact_OpenBook_KeyPadClue_C"))
  (set `self.InteractiveBookKeypadClue` _returnvalue))

(event `self.Box.OnComponentBeginOverlap`
  (params (OverlappedComponent :type "PrimitiveComponent Object Reference") (OtherActor :type "Actor Object Reference") (OtherComp :type "PrimitiveComponent Object Reference") (OtherBodyIndex :type Integer) (bFromSweep :type Boolean) (SweepResult :type "HitResult Structure (by ref)"))
  ; Prompt On screen R to open and close
  (if (== OtherActor (`GameplayStatics.GetPlayerCharacter` 0))
    (`UserWidget.AddToViewport` (`self.InteractiveBookKeypadClue`) 0)))

(event `self.Box.OnComponentEndOverlap`
  (params (OverlappedComponent :type "PrimitiveComponent Object Reference") (OtherActor :type "Actor Object Reference") (OtherComp :type "PrimitiveComponent Object Reference") (OtherBodyIndex :type Integer))
  ; Prompt On screen R to open and close
  (if (== (`GameplayStatics.GetPlayerCharacter` 0) OtherActor)
    (`Widget.RemoveFromParent` (`self.InteractiveBookKeypadClue`))))

(fn `UserConstructionScript`)