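; BP_old_book is an old book actor that shows an on-screen prompt to open it when the player is nearby.
; It creates the interact prompt widget once at BeginPlay, then adds it to the viewport when the player character enters its Box trigger and removes it on exit.
; The graph handles only the prompt, with no input or open and close logic.
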(event `self.ReceiveBeginPlay`
  ; Prompt On screen X to open and close
  (bind _returnvalue (`|CreateWidget` "/Game/OC/Widgets/WBP_Prompt_Interact_OpenBook.WBP_Prompt_Interact_OpenBook_C"))
  (set `self.InteractBookWidget` _returnvalue))

(event `self.Box.OnComponentBeginOverlap`
  (params (OverlappedComponent :type "PrimitiveComponent Object Reference") (OtherActor :type "Actor Object Reference") (OtherComp :type "PrimitiveComponent Object Reference") (OtherBodyIndex :type Integer) (bFromSweep :type Boolean) (SweepResult :type "HitResult Structure (by ref)"))
  ; Prompt On screen X to open and close
  (if (== OtherActor (`GameplayStatics.GetPlayerCharacter` 0))
    (`UserWidget.AddToViewport` (`self.InteractBookWidget`) 0)))

(event `self.Box.OnComponentEndOverlap`
  (params (OverlappedComponent :type "PrimitiveComponent Object Reference") (OtherActor :type "Actor Object Reference") (OtherComp :type "PrimitiveComponent Object Reference") (OtherBodyIndex :type Integer))
  ; Prompt On screen X to open and close
  (if (== (`GameplayStatics.GetPlayerCharacter` 0) OtherActor)
    (`Widget.RemoveFromParent` (`self.InteractBookWidget`))))

(fn `UserConstructionScript`)