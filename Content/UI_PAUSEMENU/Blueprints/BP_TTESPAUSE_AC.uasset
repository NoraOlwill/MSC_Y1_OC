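; BP_TTESPAUSE_AC is a pause menu Blueprint, likely an actor component, that toggles pausing from the IA_Pausegame input action.
; Each press plays a sound and flips an open-state flag.
; Opening creates and shows a new W_Mainmenu widget, switches to Game and UI input with the cursor visible, and pauses the game.
; Closing removes the widget, unpauses, and restores game-only input with the cursor hidden.
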(event `EnhancedInput|/Game/UI_PAUSEMENU/DEMO/Input/Actions/IA_Pausegame`
  (params (ActionValue :type Boolean) (ElapsedSeconds :type "Float (double-precision)") (TriggeredSeconds :type "Float (double-precision)") (InputAction :type "InputAction Object Reference" :default "/Game/UI_PAUSEMENU/DEMO/Input/Actions/IA_Pausegame.IA_Pausegame"))
  ;[0.0359 0.15 0.147 0.5] Pause Menu System
  (:`Started`
    (`GameplayStatics.PlaySound2D` "/Game/UI_PAUSEMENU/Audio/A_Widgetopen.A_Widgetopen" 1.0 1.0 0.0 null null)
    (if (not (`self.IsPauseMenuOpen?`))
      (set `self.IsPauseMenuOpen?` true)
      (bind _returnvalue (`|CreateWidget` "/Game/UI_PAUSEMENU/Blueprints/W_Mainmenu.W_Mainmenu_C" (`GameplayStatics.GetPlayerController` 0)))
      (bind _output_get (set `self.Pause Menu Widget` _returnvalue))
      (`UserWidget.AddToViewport` _output_get 0)
      (`WidgetBlueprintLibrary.SetInputMode_GameAndUIEx` (`GameplayStatics.GetPlayerController` 0) (`self.Pause Menu Widget`))
      (set `PlayerController.bShowMouseCursor` true (`GameplayStatics.GetPlayerController` 0))
      (`GameplayStatics.SetGamePaused` true)
      (else
        (set `self.IsPauseMenuOpen?` false)
        (`Widget.RemoveFromParent` (`self.Pause Menu Widget`))
        (`GameplayStatics.SetGamePaused` false)
        (`WidgetBlueprintLibrary.SetInputMode_GameOnly` (`GameplayStatics.GetPlayerController` 0))
        (set `PlayerController.bShowMouseCursor` false (`GameplayStatics.GetPlayerController` 0))))))